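; BP_PlayerController is a player controller that sets up a fixed camera view of the player character at game start.
; On BeginPlay it finds and stores the BP_Character, then spawns a CameraActor at a world-space Y and Z offset from it, using the character's yaw and a lowered pitch.
; It then makes that camera the view target, with no logic to follow the character afterwards.
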(event EventBeginPlay
  ;[0 0.4952 1] Inital fixed camera spawn
  (bind _returnvalue (Actor|GetActorOfClass "/Game/Blueprints/BP_Character.BP_Character_C"))
  (Variables|Default|SetcharacterRef _returnvalue)
  (bind _returnvalue_2 (Game|SpawnActorfromClass "/Script/Engine.CameraActor" (Math|Transform|MakeTransform (+ (.location (Transformation|GetActorTransform (Variables|Default|GetcharacterRef))) (Math|Vector|MakeVector 0.0 (Variables|Default|GetcameraDistance) (Variables|Default|GetcameraHeight))) (Math|Rotator|MakeRotator 0.0 (- (.pitch (.rotation (Transformation|GetActorTransform (Variables|Default|GetcharacterRef)))) (Variables|Default|GetcameraPitch)) (.yaw (.rotation (Transformation|GetActorTransform (Variables|Default|GetcharacterRef))))) "1.000000,1.000000,1.000000") "AlwaysSpawn" "MultiplyWithRoot" 0 0))
  (Game|Player|SetViewTargetwithBlend _returnvalue_2 0.0 "VTBlend_Linear" 0.0 false))

(fn ConstructionScript)